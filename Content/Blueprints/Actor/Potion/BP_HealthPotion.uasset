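; BP_HealthPotion is a potion pickup actor that applies an instant Gameplay Effect to an actor that touches it.
; Its Sphere overlap passes the other actor and InstantGameplayEffectClass to ApplyEffectToTarget, then destroys the potion without filtering who overlapped.
; On BeginPlay it uniformly scales PotionMesh from a base size plus a per-level increment driven by ActorLevel, so higher-level potions grow with a positive increment.
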(event OnComponentBeginOverlap(Sphere)
  (params (OverlappedComponent :type Primitive%20Component%20Object%20Reference) (OtherActor :type Actor%20Object%20Reference) (OtherComp :type Primitive%20Component%20Object%20Reference) (OtherBodyIndex :type Integer) (bFromSweep :type Boolean) (SweepResult :type Hit%20Result%20Structure%20%28by%20ref%29))
  (Class|AuraEffectActor|ApplyEffecttoTarget OtherActor (Variables|Default|GetInstantGameplayEffectClass))
  (Actor|DestroyActor))

(event EventBeginPlay
  (Transformation|SetRelativeScale3D (Variables|Default|GetPotionMesh) (Math|Conversions|ToVector(Float) (+ (* (- (Variables|Default|GetActorLevel) -1.0) (Variables|Default|GetExtraSizePerLevel)) (Variables|Default|GetBaseSize)))))

(event Collision|EventActorBeginOverlap
  (params (OtherActor :type Actor%20Object%20Reference)))

(event EventTick
  (params (DeltaSeconds :type Float%20%28single-precision%29)))

(fn ConstructionScript)